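; BP_PlayerController_E07_BA is a player controller Blueprint that gathers references to three character pawns in the level.
; On BeginPlay it looks up actors tagged Character1, Character2 and Character3, casts the first result of each to Pawn and stores it in a matching variable.
; The lookups run in sequence, so a failed cast stops the remaining assignments.
; The graph only caches these references, with no possession, switching or input logic.
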(event `self.ReceiveBeginPlay`
  (bind _outactors (`GameplayStatics.GetAllActorsWithTag` "Character1"))
  (bind _aspawn (cast `Pawn` (`|GetArrayItem` _outactors)))
  (set `self.Character1` _aspawn)
  (bind _outactors_2 (`GameplayStatics.GetAllActorsWithTag` "Character2"))
  (bind _aspawn_2 (cast `Pawn` (`|GetArrayItem` _outactors_2)))
  (set `self.Character2` _aspawn_2)
  (bind _outactors_3 (`GameplayStatics.GetAllActorsWithTag` "Character3"))
  (bind _aspawn_3 (cast `Pawn` (`|GetArrayItem` _outactors_3)))
  (set `self.Character3` _aspawn_3))

(fn `UserConstructionScript`)